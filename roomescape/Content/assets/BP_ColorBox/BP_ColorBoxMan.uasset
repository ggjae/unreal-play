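; BP_ColorBoxMan manages a four-box sequence puzzle, checking the order in which its color boxes are hit against a correct answer.
; Each box's OnCubeHit event appends that box's ID to an input array.
; On the fourth input, the IDs combine into a four-digit number for comparison, firing an OnAnswerIsRight or OnAnswerIsWrong dispatcher.
; A wrong answer also resets all four boxes and the input.
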(event Custom|onhitcube1
  (CallFunction|AddUserInput 1))

(event Custom|onhitcube2
  (CallFunction|AddUserInput 2))

(event Custom|onhitcube3
  (CallFunction|AddUserInput 3))

(event Custom|onhitcube4
  (CallFunction|AddUserInput 4))

(event EventBeginPlay
  (EventDispatchers|BindEventtoOnCubeHit (Variables|Default|GetCbox1) (delegate Custom|onhitcube1))
  (EventDispatchers|BindEventtoOnCubeHit (Variables|Default|GetCbox2) (delegate Custom|onhitcube2))
  (EventDispatchers|BindEventtoOnCubeHit (Variables|Default|GetCbox3) (delegate Custom|onhitcube3))
  (EventDispatchers|BindEventtoOnCubeHit (Variables|Default|GetCbox4) (delegate Custom|onhitcube4)))

(fn ConstructionScript)

(fn AddUserInput
  (params (CubeID :type Integer))
  (Utilities|Array|SetArrayElem (Variables|Default|Getarruserinput) (Variables|Default|Getarrindex) CubeID)
  (bind _output_get (Variables|Default|Setarrindex (+ (Variables|Default|Getarrindex) 1)))
  (if (== _output_get 4)
    (Development|PrintText "네개 다 맞춤")
    (bind _returnvalue (CallFunction|Makefourdigit))
    (if (== _returnvalue (Variables|Default|Getcorrectanswer))
      (Default|CallOnAnswerIsRight)
      (else
        (Default|CallOnAnswerIsWrong)
        (Default|ResetData (Variables|Default|GetCbox1))
        (Default|ResetData (Variables|Default|GetCbox2))
        (Default|ResetData (Variables|Default|GetCbox3))
        (Default|ResetData (Variables|Default|GetCbox4))
        (CallFunction|ResetInput)))))

(fn Makefourdigit
  (bind _arruserinput (Variables|Default|Getarruserinput))
  (return (+ (* (Utilities|Array|Get(acopy) _arruserinput) 1000) (* (Utilities|Array|Get(acopy) _arruserinput 1) 100) (* (Utilities|Array|Get(acopy) _arruserinput 2) 10) (Utilities|Array|Get(acopy) _arruserinput 3))))

(fn ResetInput
  (Utilities|Array|SetArrayElem (Variables|Default|Getarruserinput) 0 -1)
  (Utilities|Array|SetArrayElem (Variables|Default|Getarruserinput) 1 -1)
  (Utilities|Array|SetArrayElem (Variables|Default|Getarruserinput) 2 -1)
  (Utilities|Array|SetArrayElem (Variables|Default|Getarruserinput) 3 -1)
  (Variables|Default|Setarrindex 0))