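; BP_4colorswitch is an interactable four-color switch puzzle actor that checks a player's answer entered through a BP_UI widget.
; Overlapping its box collision shows a text prompt and enables input, so releasing F opens the widget with mouse cursor and UI-only input.
; The widget's answer event is compared to CorrectAnswer, firing OnAnswerIsRight or OnAnswerIsWrong.
; Only a wrong answer clears IsShowUI, allowing the widget to be opened again.
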(event OnComponentBeginOverlap(boxcollision)
  (params (OverlappedComponent :type Primitive%20Component%20Object%20Reference) (OtherActor :type Actor%20Object%20Reference) (OtherComp :type Primitive%20Component%20Object%20Reference) (OtherBodyIndex :type Integer) (bFromSweep :type Boolean) (SweepResult :type Hit%20Result%20Structure%20%28by%20ref%29))
  (Rendering|SetVisibility (Variables|Default|GetTextRender) true false)
  (Input|EnableInput (Game|GetPlayerController 0)))

(event OnComponentEndOverlap(boxcollision)
  (params (OverlappedComponent :type Primitive%20Component%20Object%20Reference) (OtherActor :type Actor%20Object%20Reference) (OtherComp :type Primitive%20Component%20Object%20Reference) (OtherBodyIndex :type Integer))
  (Rendering|SetVisibility (Variables|Default|GetTextRender) false false)
  (Input|DisableInput (Game|GetPlayerController 0)))

(event Custom|OnUserAnswer
  (params (UserInput :type Integer))
  (if (== (Variables|Default|GetCorrectAnswer) UserInput)
    (Default|CallOnAnswerIsRight UserInput)
    (else
      (Default|CallOnAnswerIsWrong UserInput)
      (Variables|Default|Setis_show_UI false))))

(event EventBeginPlay
  (Utilities|FlowControl|Sequence
    (:then_0
      (bind _returnvalue (UserInterface|CreateWidget "/Game/Maps/level2/BP_UI.BP_UI_C"))
      (Variables|Default|SetswitchUI _returnvalue))
    (:then_1
      (EventDispatchers|BindEventtoOnUserAnswer (Variables|Default|GetswitchUI) (delegate Custom|OnUserAnswer)))))

(event Collision|EventActorBeginOverlap
  (params (OtherActor :type Actor%20Object%20Reference)))

(event EventTick
  (params (DeltaSeconds :type Float%20%28single-precision%29)))

(event Input|KeyboardEvents|F
  (params (Key :type Key%20Structure :default "None"))
  (bind _returnvalue (Game|GetPlayerController 0))
  (:Released
    (if (not (Variables|Default|Getis_show_UI))
      (UserInterface|Viewport|AddtoViewport (Variables|Default|GetswitchUI) 0)
      (Variables|Default|Setis_show_UI true)
      (Variables|/Script/Engine.PlayerController|SetbShowMouseCursor _returnvalue true)
      (Input|SetInputModeUIOnly _returnvalue 0 "DoNotLock"))))

(fn ConstructionScript)