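; BP_Colorbox is a colored cube actor whose glow goes dark when it is hit.
; The construction script creates a dynamic material on the Cube, and BeginPlay applies the instance's color and brightness variables to it.
; A component hit zeroes the brightness parameter and calls OnCubeHit.
; ResetData restores a fixed brightness, independent of the starting Right value.
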(event OnComponentHit(Cube)
  (params (HitComponent :type Primitive%20Component%20Object%20Reference) (OtherActor :type Actor%20Object%20Reference) (OtherComp :type Primitive%20Component%20Object%20Reference) (NormalImpulse :type Vector :default "0, 0, 0") (Hit :type Hit%20Result%20Structure%20%28by%20ref%29))
  (Rendering|Material|SetScalarParameterValue (Variables|Default|GetMaterial_instance) "right" 0.0 :!class /Script/Engine.MaterialInstanceDynamic) ; 빛의 밝기 어둡게
  (Default|CallOnCubeHit))

(event EventBeginPlay
  (Rendering|Material|SetVectorParameterValue (Variables|Default|GetMaterial_instance) "defaultcolor" (Math|Conversions|ToLinearColor(Color) (Variables|Default|Getdefaultcolor)) :!class /Script/Engine.MaterialInstanceDynamic) ; 색상 변경
  (Rendering|Material|SetScalarParameterValue (Variables|Default|GetMaterial_instance) "right" (Variables|Default|Getright) :!class /Script/Engine.MaterialInstanceDynamic))

(event Collision|EventActorBeginOverlap
  (params (OtherActor :type Actor%20Object%20Reference)))

(event EventTick
  (params (DeltaSeconds :type Float%20%28single-precision%29)))

(fn ConstructionScript
  (bind _returnvalue (Rendering|Material|CreateDynamicMaterialInstance (Variables|Default|GetCube) 0 0 "None" :!class /Script/Engine.PrimitiveComponent))
  (Variables|Default|SetMaterial_instance _returnvalue))

(fn ResetData
  (Rendering|Material|SetScalarParameterValue (Variables|Default|GetMaterial_instance) "right" 2.0 :!class /Script/Engine.MaterialInstanceDynamic))